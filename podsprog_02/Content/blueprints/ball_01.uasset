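; Player-controlled ball that rolls by physics torque and restarts on taking damage.
; Both movement input axes feed one torque call on the sphere, applying the axis value times a strength multiplier to X and Y as an acceleration change.
; The camera fades in at BeginPlay; any damage fades it out, then opens level "01" after a short delay.
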(event Game|Damage|EventAnyDamage
  (params (Damage :type Float%20%28single-precision%29) (DamageType :type Damage%20Type%20Object%20Reference) (InstigatedBy :type Controller%20Object%20Reference) (DamageCauser :type Actor%20Object%20Reference))
  (CameraFades|StartCameraFade :self (Game|GetPlayerCameraManager 0) :FromAlpha 0.0 :ToAlpha 1.0 :Duration 1.0 :bHoldWhenFinished true)
  (Utilities|FlowControl|Delay 1.0)
  (Game|OpenLevel(byName) "01"))

(event EventBeginPlay
  (CameraFades|StartCameraFade :self (Game|GetPlayerCameraManager 0) :FromAlpha 1.0 :Duration 1.0 :bHoldWhenFinished true))

(event Input|AxisEvents|InputAxismoveforwardback
  (params (AxisValue :type Float%20%28single-precision%29))
  (bind _strmultiply (Variables|ballproperties|Getstrmultiply))
  (Class|PrimitiveComponent|AddTorqueinRadians (Variables|Default|GetSphere) (Math|Vector|MakeVector (* (stale Input|AxisEvents|InputAxismoveleftright AxisValue) _strmultiply) (* AxisValue _strmultiply) 0.0) "None" true))

(event Input|AxisEvents|InputAxismoveleftright
  (params (AxisValue :type Float%20%28single-precision%29))
  (bind _strmultiply (Variables|ballproperties|Getstrmultiply))
  (Class|PrimitiveComponent|AddTorqueinRadians (Variables|Default|GetSphere) (Math|Vector|MakeVector (* AxisValue _strmultiply) (* (stale Input|AxisEvents|InputAxismoveforwardback AxisValue) _strmultiply) 0.0) "None" true))

(fn ConstructionScript)